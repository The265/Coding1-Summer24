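; Falling platform actor that drops shortly after the player character steps on it, then returns to its starting position.
; A box overlap starts a Ready-gated sequence: a one-second warning, physics simulation on the cube for the fall, then a delayed reset.
; The reset disables physics and uses a timeline to lerp from the fallen transform back to the one saved at BeginPlay.
; Material swaps show each state.
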(event `self.ReceiveBeginPlay`
  (set `self.StartingTransform` (`SceneComponent.K2_GetComponentToWorld` (`self.Cube`))))

(event `self.Box.OnComponentBeginOverlap`
  (params (OverlappedComponent :type "PrimitiveComponent Object Reference") (OtherActor :type "Actor Object Reference") (OtherComp :type "PrimitiveComponent Object Reference") (OtherBodyIndex :type Integer) (bFromSweep :type Boolean) (SweepResult :type "HitResult Structure (by ref)"))
  (cast `/Game/BluePrints/BP_ThirdPersonCharacterCustom` OtherActor)
  (`self.Activate`))

(event `Activate`
  ;[1 0.6734 0.5831] Activating platform when a player stands on it.
  (if (`self.Ready`)
    (`KismetSystemLibrary.PrintString` "One second Left" true true (struct :`R` 1.0 :`B` 0.630471 :`A` 1.0))
    (set `self.Ready` false)
    (`PrimitiveComponent.SetMaterial` (`self.Cube`) 0 "/Game/Materials/MI_PlatformActivated.MI_PlatformActivated")
    (`KismetSystemLibrary.Delay` 1.0)
    (`self.Drop`)))

(event `Drop`
  ;[1 0.5394 0.3987] Platform Drops
  (`KismetSystemLibrary.PrintString` "Dropping" true true (struct :`R` 1.0 :`B` 0.702882 :`A` 1.0))
  (`PrimitiveComponent.SetSimulatePhysics` (`self.Cube`) true)
  (`PrimitiveComponent.SetMaterial` (`self.Cube`) 0 "/Game/Materials/MI_PlatformFalling.MI_PlatformFalling")
  (`KismetSystemLibrary.Delay` 3.0)
  (`self.Reset`))

(event `Reset`
  ;[0.644 0.878 1] Platform Resets
  (`KismetSystemLibrary.PrintString` "Restarting")
  (set `self.ResetTransform` (`SceneComponent.K2_GetComponentToWorld` (`self.Cube`)))
  (`PrimitiveComponent.SetSimulatePhysics` (`self.Cube`) false)
  (`PrimitiveComponent.SetMaterial` (`self.Cube`) 0 "/Game/Materials/MI_PlatformReseting.MI_PlatformReseting")
  (bind (_direction _newtrack_0) (`Timeline|Go Back To Start` :!via `PlayFromStart`)
    (:`Update`
      (bind (_returnvalue_location _returnvalue_rotation) (`KismetMathLibrary.BreakTransform` (`KismetMathLibrary.TLerp` (`self.ResetTransform`) (`self.StartingTransform`) _newtrack_0)))
      (`SceneComponent.K2_SetWorldLocationAndRotation` (`self.Cube`) _returnvalue_location _returnvalue_rotation false false))
    (:`Finished`
      (set `self.Ready` true)
      (`PrimitiveComponent.SetMaterial` (`self.Cube`) 0 "/Game/Materials/MI_PlatformReady.MI_PlatformReady"))))

(fn `UserConstructionScript`)